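; SpawnSourceBP is a spawner actor that scatters TundraRockBP rocks over the surface below it at BeginPlay.
; A loop driven by NumberOfActors traces from SourcePlane toward randomly offset points far below on the Visibility channel.
; Each rock spawns at the hit location, without a hit check, at random uniform scale.
; Its random rotation value feeds a direction vector's Y, so yaw is effectively constant.
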(event `self.ReceiveBeginPlay`
  (bind _posmin (`self.PosMin`))
  (bind _posmax (`self.PosMax`))
  (bind _returnvalue (`SceneComponent.K2_GetComponentLocation` (`self.SourcePlane`)))
  (for _ (range (+ (`self.NumberOfActors`) 1))
    (bind _outhit (`KismetSystemLibrary.LineTraceSingle` _returnvalue (+ (`KismetMathLibrary.MakeVector` (`KismetMathLibrary.RandomFloatInRange` _posmin _posmax) (`KismetMathLibrary.RandomFloatInRange` _posmin _posmax) -10000.0) _returnvalue) "TraceTypeQuery1"))
    (`|SpawnActorFromClass` "/Game/Blueprints/TundraRockBP.TundraRockBP_C" (`KismetMathLibrary.MakeTransform` (`.Location` (`GameplayStatics.BreakHitResult` _outhit)) (`KismetMathLibrary.Conv_VectorToRotator` (`KismetMathLibrary.MakeVector` 0.0 (`KismetMathLibrary.RandomFloatInRange` 0.0 360.0))) (`KismetMathLibrary.Conv_DoubleToVector` (`KismetMathLibrary.RandomFloatInRange` 0.25 5.0))) "Undefined" "OverrideRootScale" null null)))

(event `self.ReceiveTick`
  (params (DeltaSeconds :type "Float (single-precision)")))

(fn `UserConstructionScript`)