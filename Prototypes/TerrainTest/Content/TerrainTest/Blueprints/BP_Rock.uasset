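; BP_Rock is a construction-time scatter actor that places a cluster of rock static meshes.
; Its construction script loops NumOfRocks times, adding a mesh component at a random horizontal offset scaled by Modifier, with Z fixed at zero.
; Each iteration also sets the whole actor's scale uniformly from ScaleRange, rather than scaling individual meshes.
; The event graph holds only disabled placeholder events, so there is no runtime logic.
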(fn `UserConstructionScript`
  (bind _scalerange (`self.ScaleRange`))
  (for _ (range 1 (+ (`self.NumOfRocks`) 1))
    (`self.SetActorScale3D` (`KismetMathLibrary.MakeVector` _scalerange _scalerange _scalerange))
    (`AddComponent|NODE_AddStaticMeshComponent-0` :`RelativeTransform` (`KismetMathLibrary.Conv_VectorToTransform` (`KismetMathLibrary.MakeVector` (.x (* (`KismetMathLibrary.RandomUnitVector`) (`self.Modifier`))) (.y (* (`KismetMathLibrary.RandomUnitVector`) (`self.Modifier`))))))))